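; BP_sticky_note_interactor is a level actor that lets the player read a group of sticky notes through a UI widget.
; On BeginPlay it creates a Sticky_note_widget for its NoteGroup.
; Opening shows the widget with cursor and UI-only input, and calls SetSprite on its PaperSprite.
; Closing restores game input, makes the referenced Lever usable and destroys the actor, which a separate event can also do directly.
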(event Custom|Close%20Sticky%20Notes
  (bind _returnvalue (Game|GetPlayerController 0))
  (Widget|RemovefromParent (Variables|Default|GetUI))
  (Variables|/Script/Engine.PlayerController|SetbShowMouseCursor _returnvalue false)
  (Input|SetInputModeGameOnly _returnvalue false)
  (Default|SetUsable (Variables|Default|Getlever))
  (Actor|DestroyActor))

(event Custom|Open%20Sticky%20Notes
  (bind _returnvalue (Game|GetPlayerController 0))
  (UserInterface|Viewport|AddtoViewport (Variables|Default|GetUI) 0)
  (Variables|/Script/Engine.PlayerController|SetbShowMouseCursor _returnvalue true)
  (Input|SetInputModeUIOnly _returnvalue 0 "DoNotLock" false)
  (Rendering|Components|Sprite|SetSprite (Variables|Default|GetPaperSprite) 0))

(event Custom|Destroy%20sticky%20note
  (Actor|DestroyActor))

(event EventBeginPlay
  (bind _returnvalue (UserInterface|CreateWidget "/Game/UI/Sticky_Note/sticky_note_widget.sticky_note_widget_C" 0 (Variables|Default|Getnote_group)))
  (Variables|Default|SetUI _returnvalue))

(fn ConstructionScript)