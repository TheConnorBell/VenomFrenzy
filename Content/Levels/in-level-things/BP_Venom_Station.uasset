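; Venom processing station that turns an animal's venom item into that animal's antivenom.
; InsertItem validates the name suffix, tints the dispensed sprite from the item data table, then flies the item along a runtime-built spline into the funnel.
; The blender then shakes with sound until a Tick countdown stops it and slides out the product.
; ResetMachine spawns the antivenom for pickup; box overlap toggles a custom-depth highlight.
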(event OnComponentBeginOverlap(Box)
  (params (OverlappedComponent :type Primitive%20Component%20Object%20Reference) (OtherActor :type Actor%20Object%20Reference) (OtherComp :type Primitive%20Component%20Object%20Reference) (OtherBodyIndex :type Integer) (bFromSweep :type Boolean) (SweepResult :type Hit%20Result%20Structure%20%28by%20ref%29))
  (bind _paperflipbook (Variables|Default|GetPaperFlipbook))
  (Rendering|SetRenderCustomDepth _paperflipbook true)
  (Rendering|SetCustomDepthStencilValue _paperflipbook 2))

(event OnComponentEndOverlap(Box)
  (params (OverlappedComponent :type Primitive%20Component%20Object%20Reference) (OtherActor :type Actor%20Object%20Reference) (OtherComp :type Primitive%20Component%20Object%20Reference) (OtherBodyIndex :type Integer))
  (Rendering|SetRenderCustomDepth (Variables|Default|GetPaperFlipbook) false))

(event Custom|Insert%20Item
  (params (item_id :type BP%20Item%20Class%20Object%20Reference))
  (bind _specific_item (Variables|/Game/Characters/Items/BP_Item_Class.BP_Item_Class_C|Getspecific_item item_id))
  (bind (_lefts _rights) (Utilities|String|Split _specific_item "-"))
  (bind _returnvalue (Utilities|String|Append _lefts "-antivenom"))
  (if (Variables|Default|Getis_usable)
    (if (Utilities|Enum|NotEqual(Enum) _specific_item "empty_bottle")
      (Development|PrintString _rights)
      (switch string _rights
        (:venom
          (bind _output_get (Variables|Default|Setcurrently_using item_id))
          (Variables|Default|Setis_usable false)
          (Variables|Default|Setspecific_animal _lefts)
          (Variables|Default|SetitemToSpawn _returnvalue)
          (bind _returnvalue_2 (Utilities|GetDataTableRow "/Game/Characters/Items/Item_Datatable.Item_Datatable" (Utilities|String|StringToName _returnvalue))
            (:then
              (Sprite|SetSpriteColor (Variables|Default|GetdispensedSprite) (Math|Conversions|ToLinearColor(Color) (.fluid_colour _returnvalue_2)))
              (Default|TakeItem _output_get)
              (bind _asbp_player_character (Utilities|Casting|CastToBP_PlayerCharacter (Game|GetPlayerCharacter 0)))
              (Default|RemoveItem _asbp_player_character)
              (Variables|Default|Setitem_is_moving_to_funnel true)
              (Variables|Default|Setstart_location (Transformation|GetActorLocation (Variables|Default|Getcurrently_using)))
              (bind _returnvalue_3 (AddComponent|AddSplineComponent false))
              (bind _output_get_2 (Variables|Default|Settemp_spline _returnvalue_3))
              (Spline|SetLocationatSplinePoint _output_get_2 0 (Variables|Default|Getstart_location) "Local" true)
              (Spline|SetLocationatSplinePoint _output_get_2 1 (+ (/ (+ (Variables|Default|Getstart_location) (Transformation|GetWorldLocation (Variables|Default|GetaboveFunnelPoint1))) "2.000000,2.000000,2.000000") "0.000000,0.000000,100.000000") "Local" true)
              (Spline|AddSplinePoint _output_get_2 (Transformation|GetWorldLocation (Variables|Default|GetaboveFunnelPoint1)) "Local" true)
              (Spline|AddSplinePoint _output_get_2 (Transformation|GetWorldLocation (Variables|Default|GetaboveFunnelPoint)) "Local" true)
              (Spline|SetSplinePointType _output_get_2 0 "Curve" true)
              (Spline|SetSplinePointType _output_get_2 1 "Curve" true)
              (Spline|SetSplinePointType _output_get_2 2 "Curve" true)
              (Spline|SetSplinePointType _output_get_2 3 "Constant" true)
              (Spline|UpdateSpline _output_get_2)
              (CallFunction|AnimateMovement))))))))

(event Custom|reset%20machine
  (params (holding_new_item :type Boolean))
  (Variables|Default|Setitem_pickup_ready false)
  (Variables|Default|Setis_usable true)
  (Transformation|SetRelativeLocation (Variables|Default|GetdispensedSprite) "0.000000,-10.229084,-25.000000" false false)
  (bind _returnvalue (Game|SpawnActorfromClass "/Game/Characters/Items/BP_Item_Class.BP_Item_Class_C" (Transformation|GetActorTransform (Game|GetPlayerCharacter 0)) "AlwaysSpawn" "MultiplyWithRoot" 0 (Variables|Default|GetitemToSpawn) true (Variables|Default|Getspecific_animal) "0.000000,0.000000,0.000000" "None" false 0 true 0))
  (Development|PrintString (Variables|/Game/Characters/Items/BP_Item_Class.BP_Item_Class_C|Getspecific_item _returnvalue))
  (Default|PickupAnimal _returnvalue holding_new_item))

(event Custom|Run%20Machine
  (Sprite|SetFlipbook (Variables|Default|GetPaperFlipbook) "/Game/Assets/Environment/Blender_On.Blender_On")
  (Variables|Default|Setmachine_is_running true)
  (bind _returnvalue (Audio|SpawnSoundatLocation "/Game/Assets/Sounds/large-fan-running-81736.large-fan-running-81736" (Variables|Default|Getstart_location) "0, 0, 0" 1.0 1.0 0.0 0 0))
  (bind _alpha (Timeline|machine_shake Play)
    (:Update
      (Transformation|SetRelativeRotation (Variables|Default|GetPaperFlipbook) (Math|Rotator|MakeRotator 0.0 (* _alpha 5.0) 0.0) false false))
    (:Finished
      (if (Variables|Default|Getmachine_is_running)
        (Timeline|machine_shake PlayFromStart)
        (else
          (Audio|Components|Audio|StopDelayed _returnvalue 0.0))))))

(event Custom|animate%20Movement
  (bind _temp_spline (Variables|Default|Gettemp_spline))
  (bind _alpha (Timeline|Follow%20Spline PlayFromStart)
    (:Update
      (Transformation|SetActorLocation (Variables|Default|Getcurrently_using) (Spline|GetLocationatDistanceAlongSpline _temp_spline (* _alpha (Spline|GetSplineLength _temp_spline)) "Local") false false))
    (:Finished
      (Actor|DestroyActor (Variables|Default|Getcurrently_using))
      (Variables|Default|Setitem_is_moving_to_funnel false)
      (CallFunction|RunMachine))))

(event Custom|stop%20Machine
  (bind _dispensedsprite (Variables|Default|GetdispensedSprite))
  (Variables|Default|Setmachine_is_running false)
  (Variables|Default|Setmachine_time_remaining 3.0)
  (Sprite|SetFlipbook (Variables|Default|GetPaperFlipbook) "/Game/Assets/Environment/Blender_Off.Blender_Off")
  (Utilities|FlowControl|Delay 0.2)
  (bind _newtrack_0 (Timeline|Timeline Play)
    (:Update
      (Transformation|AddLocalOffset _dispensedsprite (- (Math|Vector|MakeVector 0.0 -10.229084 (+ (* (- (Math|Conversions|ToFloat(Integer) "-43.247465") -25.0) _newtrack_0) -25.0)) (Variables|/Script/Engine.SceneComponent|GetRelativeLocation _dispensedsprite)) false false))
    (:Finished
      (Variables|Default|Setitem_pickup_ready true))))

(event EventTick
  (params (DeltaSeconds :type Float%20%28single-precision%29))
  (if (Variables|Default|Getmachine_is_running)
    (if (<= (Variables|Default|Getmachine_time_remaining) 0.0)
      (CallFunction|StopMachine)
      (else
        (Variables|Default|Setmachine_time_remaining (- (Variables|Default|Getmachine_time_remaining) DeltaSeconds))))))

(fn ConstructionScript)