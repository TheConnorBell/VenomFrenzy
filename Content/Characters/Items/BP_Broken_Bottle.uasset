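; BP_Broken_Bottle is a short-lived Paper2D actor for a broken bottle, with optional coloured fluid.
; On BeginPlay it tints the second sprite with FluidColour if Fluid is set, or clears that sprite otherwise.
; A timeline then drives the first sprite's local vertical offset from a scaled curve, and the actor destroys itself when the timeline finishes.
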(event EventBeginPlay
  (bind _papersprite1 (Variables|Default|GetPaperSprite1))
  (if (Variables|Default|Getfluid)
    (Sprite|SetSpriteColor (Variables|Default|GetPaperSprite2) (Math|Conversions|ToLinearColor(Color) (Variables|Default|Getfluid_colour)))
    (bind _newtrack_0 (Timeline|Timeline Play)
      (:Update
        (Transformation|AddLocalOffset _papersprite1 (- (Math|Vector|MakeVector 0.0 0.0 (* _newtrack_0 16.0)) (Variables|/Script/Engine.SceneComponent|GetRelativeLocation _papersprite1)) false true))
      (:Finished
        (Actor|DestroyActor)))
    (else
      (Rendering|Components|Sprite|SetSprite (Variables|Default|GetPaperSprite2) 0)
      (Timeline|Timeline Play))))

(fn ConstructionScript)