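; Base item actor that the player picks up, carries in the inventory and hands to crafting stations.
; Pickup disables collision, attaches the item above the player and adds it to inventory; hold status toggles scale to show or hide it.
; Change_Item sets the type and animal fields, then pulls the sprite from the item DataTable, tinting filled bottles by fluid colour.
; TakeItem detaches it for crafting, keeping collision off.
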(event Custom|Take%20Item
  (Transformation|DetachFromActor "KeepWorld" "KeepWorld" "KeepWorld")
  (Variables|Default|SetBeing_Held false)
  (Transformation|SetActorLocation (+ (.location (Transformation|GetActorTransform (Game|GetPlayerCharacter 0))) "0.000000,0.000000,160.000000") false true)
  (Collision|SetCollisionEnabled (Variables|Default|GetCapsuleComponent) "NoCollision")
  (Collision|SetCollisionEnabled (Variables|Default|GetInteractionRange) "NoCollision"))

(event Custom|Change_Item
  (params (New_Item_Type :type String) (is_animal_specific :type Boolean) (animal_type :type String))
  (bind _papersprite (Variables|Default|GetPaperSprite))
  (bind _output_get (Variables|Default|Setspecific_item New_Item_Type))
  (Variables|Default|Setis_animal_specific_item is_animal_specific)
  (Variables|Default|Setanimal_type animal_type)
  (bind _returnvalue (Utilities|GetDataTableRow "/Game/Characters/Items/Item_Datatable.Item_Datatable" (Utilities|String|StringToName _output_get))
    (:then
      (Rendering|Components|Sprite|SetSprite (Variables|Default|GetPaperSprite) (.sprite _returnvalue))
      (if (.is_fillled_bottle _returnvalue)
        (Sprite|SetSpriteColor _papersprite (Math|Conversions|ToLinearColor(Color) (.fluid_colour _returnvalue)))
        (else
          (Sprite|SetSpriteColor _papersprite "(R=1.000000,G=1.000000,B=1.000000,A=1.000000)"))))))

(event EventBeginPlay)

(event Collision|EventActorBeginOverlap
  (params (OtherActor :type Actor%20Object%20Reference)))

(event EventTick
  (params (DeltaSeconds :type Float%20%28single-precision%29)))

(event EventPickupAnimal
  (params (Is_Holding :type Boolean))
  (Variables|Default|SetBeing_Held Is_Holding)
  (Transformation|AttachActorToActor (Game|GetPlayerCharacter 0) "None" "KeepRelative" "KeepRelative" "KeepRelative" false)
  (Collision|SetCollisionEnabled (Variables|Default|GetCapsuleComponent) "NoCollision")
  (Collision|SetCollisionEnabled (Variables|Default|GetInteractionRange) "NoCollision")
  (bind _asbp_player_character (Utilities|Casting|CastToBP_PlayerCharacter (Game|GetPlayerCharacter 0)))
  (Default|AddtoInventory _asbp_player_character self)
  (Transformation|SetActorLocation (+ (.location (Transformation|GetActorTransform (Game|GetPlayerCharacter 0))) "0.000000,0.000000,160.000000") false true)
  (if (Variables|Default|GetBeing_Held)
    (Transformation|SetActorScale3D "1.000000,1.000000,1.000000")
    (Pawn|Components|CharacterMovement|SetMovementMode (Variables|Character|GetCharacterMovement) "MOVE_None" 0)
    (else
      (Transformation|SetActorScale3D "0, 0, 0"))))

(event EventSetHoldStatus
  (params (Is_Holding :type Boolean))
  (Variables|Default|SetBeing_Held Is_Holding)
  (if (Variables|Default|GetBeing_Held)
    (Transformation|SetActorScale3D "1.000000,1.000000,1.000000")
    (Pawn|Components|CharacterMovement|SetMovementMode (Variables|Character|GetCharacterMovement) "MOVE_None" 0)
    (else
      (Transformation|SetActorScale3D "0, 0, 0"))))

(fn ConstructionScript
  (|CallParentFunction))