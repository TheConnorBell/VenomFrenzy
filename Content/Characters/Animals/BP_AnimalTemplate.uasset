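; Base 2D flipbook animal that roams near its spawner, flees the player, hides underground and can be carried.
; Tick picks Data Table flipbooks, outlines grabbable animals via custom depth, and drives a timer-based HidingState that burrows animals inside roam range when the player is away.
; AI perception, hiding and pickup events update Blackboard keys; timelines animate burrowing and the jump out of the spawner.
; Debug range shapes always draw.
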(event OnComponentBeginOverlap(InteractionRange)
  (params (OverlappedComponent :type Primitive%20Component%20Object%20Reference) (OtherActor :type Actor%20Object%20Reference) (OtherComp :type Primitive%20Component%20Object%20Reference) (OtherBodyIndex :type Integer) (bFromSweep :type Boolean) (SweepResult :type Hit%20Result%20Structure%20%28by%20ref%29))
  (bind _asbp_player_character (Utilities|Casting|CastToBP_PlayerCharacter OtherActor))
  (Variables|Default|SetIs_Touching_Player true)
  (Default|AddTouchingAnimal _asbp_player_character self))

(event OnComponentEndOverlap(InteractionRange)
  (params (OverlappedComponent :type Primitive%20Component%20Object%20Reference) (OtherActor :type Actor%20Object%20Reference) (OtherComp :type Primitive%20Component%20Object%20Reference) (OtherBodyIndex :type Integer))
  (bind _asbp_player_character (Utilities|Casting|CastToBP_PlayerCharacter OtherActor))
  (Variables|Default|SetIs_Touching_Player false)
  (Default|RemoveTouchingAnimal _asbp_player_character self))

(event OnTargetPerceptionUpdated(AIPerception)
  (params (Actor :type Actor%20Object%20Reference) (Stimulus :type AI%20Stimulus%20Structure))
  (bind _returnvalue (Game|GetPlayerCharacter 0))
  (bind _charactermovement (Variables|Character|GetCharacterMovement))
  (bind _paperflipbook (Variables|Default|GetPaperFlipbook))
  (bind _returnvalue_2 (Transformation|GetDistanceTo _returnvalue))
  (bind _asbp_player_character (Utilities|Casting|CastToBP_PlayerCharacter Actor))
  (Utilities|IsValid _asbp_player_character
    (:Is%20Valid
      (AI|Components|Blackboard|SetValueasBool (AI|GetBlackboard 0) (Utilities|Name|MakeLiteralName "Is_Fleeing") (or (.bsuccessfullysensed Stimulus) (or (<= _returnvalue_2 (Variables|Default|GetRoam_Range)) (and (<= _returnvalue_2 9.6e+02) (Variables|Default|Getfleeing)))))
      (Variables|Default|Setfleeing (or (.bsuccessfullysensed Stimulus) (or (<= _returnvalue_2 (Variables|Default|GetRoam_Range)) (and (<= _returnvalue_2 9.6e+02) (Variables|Default|Getfleeing)))))
      (if (or (.bsuccessfullysensed Stimulus) (or (<= _returnvalue_2 (Variables|Default|GetRoam_Range)) (and (<= _returnvalue_2 9.6e+02) (Variables|Default|Getfleeing))))
        (Variables|/Script/Engine.CharacterMovementComponent|SetMaxWalkSpeed _charactermovement 3e+02)
        (Components|Timeline|SetPlayRate _paperflipbook 2.0)
        (else
          (Variables|/Script/Engine.CharacterMovementComponent|SetMaxWalkSpeed _charactermovement 1e+02)
          (Components|Timeline|SetPlayRate _paperflipbook 1.0)))
      (AI|Navigation|StopMovement (AI|GetAIController self)))))

(event Custom|Pickup_Animal
  (params (Is_Holding :type Boolean))
  (Variables|Default|SetBeing_Held Is_Holding)
  (if (Utilities|Enum|Equal(Enum) (Utilities|GetClassDisplayName (Variables|Default|GetAIControllerClass)) (Utilities|GetClassDisplayName "/Game/Characters/Animals/BP_Animal_Controller.BP_Animal_Controller_C"))
    (AI|Components|Blackboard|SetValueasBool (AI|GetBlackboard 0) (Utilities|Name|MakeLiteralName "Is_Being_Held") true)
    (AI|Navigation|StopMovement (AI|GetAIController self)))
  (Transformation|AttachActorToActor (Game|GetPlayerCharacter 0) "None" "KeepRelative" "KeepRelative" "KeepRelative" false)
  (Collision|SetCollisionEnabled (Variables|Collision|GetCapsuleComponent) "NoCollision")
  (Collision|SetCollisionEnabled (Variables|Default|GetInteractionRange) "NoCollision")
  (bind _asbp_player_character (Utilities|Casting|CastToBP_PlayerCharacter (Game|GetPlayerCharacter 0)))
  (Default|AddtoInventory _asbp_player_character self)
  (Transformation|SetActorLocation (+ (.location (Transformation|GetActorTransform (Game|GetPlayerCharacter 0))) "0.000000,0.000000,192.000000") false true)
  (if (Variables|Default|GetBeing_Held)
    (Transformation|SetActorScale3D "1.000000,1.000000,1.000000")
    (Pawn|Components|CharacterMovement|SetMovementMode (Variables|Character|GetCharacterMovement) "MOVE_None" 0)
    (else
      (Transformation|SetActorScale3D "0, 0, 0"))))

(event Custom|Drop_Animal
  (bind _charactermovement (Variables|Character|GetCharacterMovement))
  (if (Utilities|Enum|Equal(Enum) (Utilities|GetClassDisplayName (Variables|Default|GetAIControllerClass)) (Utilities|GetClassDisplayName "/Game/Characters/Animals/BP_Animal_Controller.BP_Animal_Controller_C"))
    (AI|Components|Blackboard|SetValueasBool (AI|GetBlackboard 0) (Utilities|Name|MakeLiteralName "Is_Being_Held") false))
  (Transformation|DetachFromActor "KeepWorld" "KeepWorld" "KeepWorld")
  (Collision|SetCollisionEnabled (Variables|Collision|GetCapsuleComponent) "QueryOnly")
  (Collision|SetCollisionEnabled (Variables|Default|GetInteractionRange) "QueryOnly")
  (Variables|Default|SetBeing_Held false)
  (Transformation|SetActorLocation (+ (.location (Transformation|GetActorTransform (Game|GetPlayerCharacter 0))) "10.000000,-10.000000,200.000000") false true)
  (Pawn|Components|CharacterMovement|SetMovementMode _charactermovement "MOVE_Falling" 0)
  (Variables|/Script/Engine.CharacterMovementComponent|SetbRunPhysicsWithNoController _charactermovement true))

(event Custom|Unhide_Animal
  (params (unhide_forward_jump_direction :type Integer) (unhide_sideways_jump_direction :type Integer))
  (Default|SetShakingStatus (Variables|Default|Getspawner) false)
  (CallFunction|StopBurrowing)
  (Transformation|SetActorLocation (Transformation|GetActorLocation (Variables|Default|Getspawner)) false false)
  (Transformation|SetActorScale3D "0.500000,0.500000,0.500000")
  (Variables|/Script/Engine.CharacterMovementComponent|SetGravityScale (Variables|Character|GetCharacterMovement) 1.0)
  (Variables|Default|Sethiding_state 4)
  (bind (_direction _scale _movement) (Timeline|unhide_animal_timeline PlayFromStart)
    (:Update
      (Transformation|SetActorScale3D (Math|Vector|MakeVector (+ (/ _scale 2.0) 0.5) (+ (/ _scale 2.0) 0.5) (+ (/ _scale 2.0) 0.5)))
      (Transformation|SetActorLocation (+ (Math|Vector|MakeVector (* (* _scale 5e+02) unhide_sideways_jump_direction) (* (* _scale 5e+02) unhide_forward_jump_direction) (* _movement 1.5e+02)) (+ (Transformation|GetActorLocation (Variables|Default|Getspawner)) "0.000000,0.000000,88.000000")) false true))
    (:Finished
      (AI|Components|Blackboard|SetValueasBool (AI|GetBlackboard 0) (Utilities|Name|MakeLiteralName "Is_Hiding") false)
      (Variables|Default|Setis_grabable true))))

(event Custom|Set%20Spawner%20Reference
  (params (NewParam :type BP%20Animal%20Spawner%20Object%20Reference))
  (Variables|Default|Setspawner NewParam))

(event Custom|Set_Hold_Status
  (params (Is_Holding :type Boolean))
  (Variables|Default|SetBeing_Held Is_Holding)
  (Transformation|SetActorLocation (+ (.location (Transformation|GetActorTransform (Game|GetPlayerCharacter 0))) "0.000000,0.000000,192.000000") false true)
  (if (Variables|Default|GetBeing_Held)
    (Transformation|SetActorScale3D "1.000000,1.000000,1.000000")
    (Pawn|Components|CharacterMovement|SetMovementMode (Variables|Character|GetCharacterMovement) "MOVE_None" 0)
    (else
      (Transformation|SetActorScale3D "0, 0, 0"))))

(event Custom|Set_Hiding_Animal_Status
  (bind _returnvalue (AI|GetBlackboard 0))
  (Variables|Default|Setis_grabable false)
  (Default|SetShakingStatus (Variables|Default|Getspawner) true)
  (Variables|Default|Sethiding_state 1)
  (Variables|/Script/Engine.CharacterMovementComponent|SetGravityScale (Variables|Character|GetCharacterMovement) 0.0)
  (bind _output_get (Variables|Default|SetRoam_Range 1e+02))
  (Utilities|IsValid _returnvalue
    (:Is%20Valid
      (AI|Components|Blackboard|SetValueasBool _returnvalue (Utilities|Name|MakeLiteralName "Is_Hiding") true)
      (Transformation|SetActorLocation (- (Transformation|GetActorLocation (Variables|Default|Getspawner)) "0.000000,0.000000,500.000000") false true)
      (AI|Components|Blackboard|SetValueasFloat (AI|GetBlackboard 0) (Utilities|Name|MakeLiteralName "Roam_Range") _output_get))))

(event Custom|Stop_Burrowing
  (bind _returnvalue (Transformation|GetActorLocation))
  (bind _returnvalue_2 (Transformation|GetActorLocation))
  (Transformation|AddLocalOffset (Variables|Default|GetPaperFlipbook) "0, 0, 0" false false)
  (Transformation|SetActorLocation (Math|Vector|MakeVector (.x _returnvalue_2) (.y _returnvalue_2) (.z (Transformation|GetActorLocation (Variables|Default|Getspawner)))) false false)
  (Collision|SetCollisionEnabled (Variables|Collision|GetCapsuleComponent) "QueryOnly")
  (Variables|/Script/Engine.CharacterMovementComponent|SetGravityScale (Variables|Character|GetCharacterMovement) 1.0)
  (AI|Components|Blackboard|SetValueasBool (AI|GetBlackboard 0) (Utilities|Name|MakeLiteralName "Is_Hiding") false)
  (bind (_direction _burrow _shake) (Timeline|burrowing_animal Stop)
    (:Update
      (Transformation|SetActorLocation (Math|Vector|MakeVector (.x _returnvalue) (.y _returnvalue) (+ (* _burrow -1.5) (.z _returnvalue))) false true)
      (Transformation|AddLocalOffset (Variables|Default|GetPaperFlipbook) (Math|Vector|MakeVector (* _shake 2.0) 0.0 0.0) false false))
    (:Finished
      (CallFunction|SetHidingAnimalStatus))))

(event EventBeginPlay
  (bind _returnvalue (AI|GetBlackboard 0))
  (Utilities|FlowControl|Delay 0.1)
  (Utilities|IsValid _returnvalue
    (:Is%20Valid
      (AI|Components|Blackboard|SetValueasFloat _returnvalue (Utilities|Name|MakeLiteralName "Roam_Range") (Variables|Default|GetRoam_Range))
      (Variables|Default|SetInitialRotation (Transformation|GetActorRotation))
      (AI|Components|Blackboard|SetValueasBool (AI|GetBlackboard 0) (Utilities|Name|MakeLiteralName "Is_Fleeing") false)
      (Variables|Default|Setfleeing false))))

(event EventTick
  (params (DeltaSeconds :type Float%20%28single-precision%29))
  (bind _returnvalue (Transformation|GetActorLocation))
  (bind _returnvalue_2 (Transformation|GetActorLocation))
  (bind _returnvalue_3 (AI|GetBlackboard 0))
  (bind _paperflipbook (Variables|Default|GetPaperFlipbook))
  (bind _paperflipbook_2 (Variables|Default|GetPaperFlipbook))
  (Utilities|FlowControl|Sequence
    (:then_0
      (if true ; Show Debug Renders
        (Rendering|Debug|DrawDebugSphere _returnvalue_2 5e+02 12 "(R=0.057249,G=1.000000,B=0.000000,A=1.000000)" 0.0)
        (Rendering|Debug|DrawDebugSphere _returnvalue_2 1e+03 12 "(R=1.000000,G=0.000000,B=0.026037,A=1.000000)" 0.0)
        (Rendering|Debug|DrawDebugCircle (Transformation|GetActorLocation (Variables|Default|Getspawner)) (Variables|Default|GetRoam_Range) 12 "(R=0.019228,G=0.029864,B=1.000000,A=1.000000)" 0.0 0.0 "0.000000,1.000000,0.000000" "1.000000,0.000000,0.000000"))
      (Transformation|SetActorRotation (Variables|Default|GetInitialRotation))
      (bind _returnvalue_4 (Utilities|GetDataTableRow "/Game/Characters/Animals/Animal_Database.Animal_Database" (Variables|AnimalType|GetSpecificAnimal))
        (:then
          (if (Class|KismetMathLibrary|IsNearlyZero2D (Math|Conversions|ToVector2D(Vector) (Variables|/Script/Engine.MovementComponent|GetVelocity (Variables|Character|GetCharacterMovement))) 0.01)
            (Sprite|SetFlipbook _paperflipbook_2 (.idle _returnvalue_4))
            (else
              (Math|Float|CompareFloat (.x (Variables|/Script/Engine.MovementComponent|GetVelocity (Variables|Character|GetCharacterMovement))) 0.0
                (:>
                  (Sprite|SetFlipbook _paperflipbook_2 (.right_walk _returnvalue_4) :!label _label))
                (:==
                  (goto _label))
                (:<
                  (Sprite|SetFlipbook _paperflipbook_2 (.left_walk _returnvalue_4))))))
          (if (and (Variables|Default|GetIs_Touching_Player) (Variables|Default|Getis_grabable))
            (Rendering|SetRenderCustomDepth _paperflipbook true)
            (Rendering|SetCustomDepthStencilValue _paperflipbook 1)
            (else
              (Rendering|SetRenderCustomDepth _paperflipbook false))))))
    (:then_1
      (bind _output_get (Variables|Default|Setis_within_spawn_range (< (Math|Vector|VectorLength (- (Transformation|GetActorLocation) (Transformation|GetActorLocation (Variables|Default|Getspawner)))) (Variables|Default|GetRoam_Range))))
      (Utilities|IsValid _returnvalue_3
        (:Is%20Valid
          (AI|Components|Blackboard|SetValueasBool _returnvalue_3 (Utilities|Name|MakeLiteralName "Is_within_roam_range") _output_get))))
    (:then_2
      (if (and (!= (Variables|Default|Gethiding_state) 0) (!= (Variables|Default|Gethiding_state) 1))
        (if (Variables|Default|Getis_within_spawn_range)
          (if (< (Math|Vector|VectorLength (- (Transformation|GetActorLocation) (Transformation|GetActorLocation (Game|GetPlayerCharacter 0)))) 5e+02)
            (CallFunction|StopBurrowing)
            (else
              (switch int (Variables|Default|Gethiding_state)
                (:2
                  (Variables|Default|Setsinking_timer (+ DeltaSeconds (Variables|Default|Getsinking_timer)) :!label _label_2)
                  (AI|Components|Blackboard|SetValueasBool (AI|GetBlackboard 0) (Utilities|Name|MakeLiteralName "Is_Hiding") true))
                (:3
                  (Utilities|FlowControl|Sequence
                    (:then_0
                      (goto _label_2))
                    (:then_1
                      (Collision|SetCollisionEnabled (Variables|Collision|GetCapsuleComponent) "NoCollision")
                      (Variables|/Script/Engine.CharacterMovementComponent|SetGravityScale (Variables|Character|GetCharacterMovement) 0.0)
                      (bind (_direction _burrow _shake) (Timeline|burrowing_animal Play)
                        (:Update
                          (Transformation|SetActorLocation (Math|Vector|MakeVector (.x _returnvalue) (.y _returnvalue) (+ (* _burrow -1.5) (.z _returnvalue))) false true)
                          (Transformation|AddLocalOffset (Variables|Default|GetPaperFlipbook) (Math|Vector|MakeVector (* _shake 2.0) 0.0 0.0) false false))
                        (:Finished
                          (CallFunction|SetHidingAnimalStatus))))))
                (:4
                  (Variables|Default|Sethiding_state 2)))))
          (else
            (Variables|Default|Sethiding_state 4)
            (Variables|Default|Setsinking_timer 0.0)))))
    (:then_3
      (if (> (Variables|Default|Getsinking_timer) 5.0)
        (if (> (Variables|Default|Getsinking_timer) 8.0)
          (CallFunction|SetHidingAnimalStatus)
          (else
            (Variables|Default|Sethiding_state 3)))))
    (:then_4
      (if (not (< (Math|Vector|VectorLength (- (Transformation|GetActorLocation) (Transformation|GetActorLocation (Game|GetPlayerCharacter 0)))) 1.5e+03))
        (Variables|Default|Setfleeing false)
        (AI|Components|Blackboard|SetValueasBool (AI|GetBlackboard 0) (Utilities|Name|MakeLiteralName "Is_Fleeing") false)))))

(fn ConstructionScript)