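; BP_AnimalSpawner spawns one animal at its location, optionally hidden behind an animated environment sprite such as a shaking bush or bubbles.
; BeginPlay spawns BP_AnimalTemplate, assigns its species and spawner reference, applies hiding status, and picks the flipbook for the hiding environment.
; SetShakingStatus switches those flipbooks and play rates.
; Player overlap with the Box unhides an animal in a qualifying hiding state, passing jump directions.
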(event OnComponentBeginOverlap(Box)
  (params (OverlappedComponent :type Primitive%20Component%20Object%20Reference) (OtherActor :type Actor%20Object%20Reference) (OtherComp :type Primitive%20Component%20Object%20Reference) (OtherBodyIndex :type Integer) (bFromSweep :type Boolean) (SweepResult :type Hit%20Result%20Structure%20%28by%20ref%29))
  (bind _stored_animal (Variables|Animal|Getstored_animal))
  (bind _hiding_state (Variables|/Game/Characters/Animals/BP_AnimalTemplate.BP_AnimalTemplate_C|Gethiding_state _stored_animal))
  (bind _asbp_player_character (Utilities|Casting|CastToBP_PlayerCharacter OtherActor))
  (Utilities|IsValid _asbp_player_character
    (:Is%20Valid
      (if (or (== _hiding_state 1) (== _hiding_state 2))
        (Default|UnhideAnimal _stored_animal (Variables|Default|Getjump_forwards) (Variables|Default|Getjump_sideways))))))

(event Custom|Set%20Shaking%20Status
  (params (NewParam :type Boolean))
  (bind _horizontal_sprite (Variables|Default|Gethorizontal_sprite))
  (bind _horizontal_sprite_2 (Variables|Default|Gethorizontal_sprite))
  (bind _verticle_sprite (Variables|Default|Getverticle_sprite))
  (bind _verticle_sprite_2 (Variables|Default|Getverticle_sprite))
  (bind _output_get (Variables|Default|Setshaking_status NewParam))
  (if _output_get
    ;[0.15 0.15 0.15 0.5] When element should be animated
    (switch int (Variables|Default|Gethiding_environment)
      (:1
        (Sprite|SetFlipbook _verticle_sprite "/Game/Assets/Environment/shaking_bush.shaking_bush")
        (Components|Timeline|SetPlayRate _verticle_sprite 4.0))
      (:2
        (Sprite|SetFlipbook _horizontal_sprite_2 "/Game/Assets/Environment/Bubbling_Flipbook.Bubbling_Flipbook")
        (Components|Timeline|SetPlayRate _horizontal_sprite_2 4.0)))
    (else
      ;[0.15 0.15 0.15 0.5] When element shouldn't be animated
      (switch int (Variables|Default|Gethiding_environment)
        (:1
          (Sprite|SetFlipbook _verticle_sprite_2 "/Game/Assets/Environment/shaking_bush.shaking_bush")
          (Components|Timeline|SetPlayRate _verticle_sprite_2 1.0))
        (:2
          (Sprite|SetFlipbook _horizontal_sprite)
          (Components|Timeline|SetPlayRate _horizontal_sprite 1.0))))))

(event EventBeginPlay
  (bind _returnvalue (Transformation|GetActorLocation))
  (bind _horizontal_sprite (Variables|Default|Gethorizontal_sprite))
  (bind _verticle_sprite (Variables|Default|Getverticle_sprite))
  (Utilities|FlowControl|Sequence
    (:then_0
      (bind _returnvalue_2 (AI|SpawnAIFromClass "/Game/Characters/Animals/BP_AnimalTemplate.BP_AnimalTemplate_C" 0 (Math|Vector|MakeVector (.x _returnvalue) (.y _returnvalue) (.z _returnvalue)) "0, 0, 0" false 0))
      (bind _asbp_animal_template (Utilities|Casting|CastToBP_AnimalTemplate _returnvalue_2))
      (bind _output_get (Variables|Animal|Setstored_animal _asbp_animal_template))
      (Variables|/Game/Characters/Animals/BP_AnimalTemplate.BP_AnimalTemplate_C|SetSpecificAnimal _output_get (Variables|Animal|GetAnimal))
      (Default|SetSpawnerReference _output_get self)
      (if (Variables|Default|Gethiding_animal)
        (Default|SetHidingAnimalStatus _asbp_animal_template)))
    (:then_1
      (switch int (Variables|Default|Gethiding_environment)
        (:0
          (Sprite|SetFlipbook (Variables|Default|Getverticle_sprite)))
        (:1
          (Sprite|SetFlipbook _verticle_sprite "/Game/Assets/Environment/shaking_bush.shaking_bush")
          (Components|Timeline|SetPlayRate _verticle_sprite 4.0))
        (:2
          (Sprite|SetFlipbook _horizontal_sprite "/Game/Assets/Environment/Bubbling_Flipbook.Bubbling_Flipbook")
          (Components|Timeline|SetPlayRate _horizontal_sprite 4.0))))))

(fn ConstructionScript)