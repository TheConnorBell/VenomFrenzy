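; BP_Dead_Patient is an actor, apparently representing a patient who has died, that floats upward and then removes itself.
; Tick moves it straight up at a constant, frame-rate-independent speed, without sweeping for collision, while accumulating elapsed time.
; Once that time passes a few seconds, the actor destroys itself.
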(event EventTick
  (params (DeltaSeconds :type Float%20%28single-precision%29))
  (bind _returnvalue (Transformation|GetActorLocation))
  (if (> (Variables|Default|GetelapsedTime) 5.0)
    (Actor|DestroyActor)
    (else
      (Variables|Default|SetelapsedTime (+ (Variables|Default|GetelapsedTime) DeltaSeconds))
      (Transformation|SetActorLocation (Math|Vector|MakeVector (.x _returnvalue) (.y _returnvalue) (+ (* DeltaSeconds 2e+02) (.z _returnvalue))) false false))))

(fn ConstructionScript)