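; Patient spawner that runs a clinic day: spawning patients, timing, counting cures and deaths, and showing the end popup.
; BeginPlay loads level config, dialogue, bestiary and world-state data layers; gauntlet mode chains all levels' spawns into successive days.
; A one-second timer advances spawn time, skipping idle gaps.
; Tick backlogs due entries, spawns randomized or special patients into free queues, and ends the day when patients run out.
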(event Custom|start_day
  ;[0.15 0.15 0.15 0.5] Handle Timer
  (Variables|Default|Setday_started true)
  (Timeline|one%20second%20timer Play
    (:Finished
      (bind _output_get (Variables|Default|SetTime_Since_Start (+ 1.0 (Variables|Default|GetTime_Since_Start))))
      (Variables|Default|SetPatient_Spawn_Time (+ 1.0 (Variables|Default|GetPatient_Spawn_Time)))
      (Default|UpdateTimer (Variables|Default|Gettimer_widget) (Math|Float|Truncate _output_get))
      (if (Variables|Default|Getday_started)
        (Timeline|one%20second%20timer PlayFromStart)))))

(event Custom|Stop_timer
  ;[0.15 0.15 0.15 0.5] Handle Timer
  (Timeline|one%20second%20timer Stop
    (:Finished
      (bind _output_get (Variables|Default|SetTime_Since_Start (+ 1.0 (Variables|Default|GetTime_Since_Start))))
      (Variables|Default|SetPatient_Spawn_Time (+ 1.0 (Variables|Default|GetPatient_Spawn_Time)))
      (Default|UpdateTimer (Variables|Default|Gettimer_widget) (Math|Float|Truncate _output_get))
      (if (Variables|Default|Getday_started)
        (Timeline|one%20second%20timer PlayFromStart)))))

(event Custom|patient_dealt_with
  (params (cured :type Boolean))
  (Utilities|IsValid (Variables|Default|Getend_of_level_ui)
    (:Is%20Not%20Valid
      (if cured
        (bind _result (Math|Integer|IncrementInt (Variables|Default|Getcure_count))
          (:%20%20
            (Variables|Default|Setcure_count _result)))
        (else
          (bind _result_2 (Math|Integer|IncrementInt (Variables|Default|Getdeath_count))
            (:%20%20
              (bind _output_get (Variables|Default|Setdeath_count _result_2))
              (Variables|Default|Setday_finished (>= _output_get (Variables|Default|Getdeath_limit))))))))))

(event Custom|Reset_Queue_For_Gauntlet
  (params (queues :type Integer))
  (bind _output_get (Variables|Default|SetQueue_List (Variables|Default|Getfull_queue)))
  (bind (_arrayindex _arrayelement) (Utilities|Array|ReverseforEachLoop _output_get)
    (:LoopBody
      (if (not (< _arrayindex queues))
        (Utilities|Array|RemoveItem _output_get _arrayelement)))))

(event EventBeginPlay
  (bind _asbp_game_instance (Utilities|Casting|CastToBP_GameInstance (Game|GetGameInstance)))
  (if (Variables|/Game/Levels/BP_GameInstance.BP_GameInstance_C|Getis_doing_gauntlet _asbp_game_instance)
    (Variables|/Game/Levels/BP_GameInstance.BP_GameInstance_C|SetSelectedLevelID%20 _asbp_game_instance "Level_Gauntlet")
    (bind _output_get (Variables|Default|SetWorld_State_ID "World_State_3"))
    (bind _returnvalue (Utilities|GetDataTableRow "/Game/Dialogue/Patient_Dialogue_Database.Patient_Dialogue_Database" _output_get)
      (:then
        (bind _output_get_2 (Variables|Default|SetDialogue_Options _returnvalue))
        (bind _returnvalue_2 (Actor|GetActorOfClass "/Game/Levels/in-level-things/Beastiary_Interaction.Beastiary_Interaction_C"))
        (Default|LoadAnimals _returnvalue_2 (.animal_list _output_get_2))
        (bind _outrownames (DataTable|GetDataTableRowNames "/Game/Levels/Levels_Config_Table.Levels_Config_Table"))
        (for _array_element _outrownames
          (bind _returnvalue_3 (Utilities|GetDataTableRow "/Game/Levels/Levels_Config_Table.Levels_Config_Table" _array_element)
            (:then
              (Utilities|Array|AppendArray (Variables|Default|GetNPC_List) (.patient_spawns _returnvalue_3)))))
        (Development|PrintString "Hello")
        (for (_array_element_2 _array_index) (Variables|Default|GetNPC_List)
          (if (.first_patient_of_day _array_element_2)
            (Variables|Default|Settemp_gauntlet_time_increase (+ (Variables|Default|Gettemp_gauntlet_time_increase) 10000)))
          (Utilities|Array|SetArrayElem (Variables|Default|GetNPC_List) _array_index (Utilities|Struct|MakeNPC_Spawn_Config_Struct (+ (.spawn_time _array_element_2) (Variables|Default|Gettemp_gauntlet_time_increase)) (.possible_animals _array_element_2) (.first_patient_of_day _array_element_2) (.special_npc _array_element_2) (.special_npc_type _array_element_2))))
        (Variables|Default|Setfull_queue (Variables|Default|GetQueue_List))
        (bind _returnvalue_4 (Utilities|GetDataTableRow "/Game/Levels/Levels_Config_Table.Levels_Config_Table" "Level_1")
          (:then
            (CallFunction|ResetQueueforGauntlet (.queue_number _returnvalue_4))
            (Variables|Default|Setdeath_limit 0)))))
    (else
      (bind _output_get_3 (Variables|/Game/Levels/BP_GameInstance.BP_GameInstance_C|SetSelectedLevelID%20 _asbp_game_instance (Variables|/Game/Levels/BP_GameInstance.BP_GameInstance_C|GetSelectedLevelID%20 _asbp_game_instance)))
      (Development|PrintString (Utilities|String|ToString(Name) _output_get_3) true true "(R=1.000000,G=0.842870,B=0.000000,A=1.000000)" 5.0)
      (bind _returnvalue_5 (Utilities|GetDataTableRow "/Game/Levels/Levels_Config_Table.Levels_Config_Table" _output_get_3)
        (:then
          (Variables|Default|SetNPC_List (.patient_spawns _returnvalue_5))
          (Variables|Default|Setfull_queue (Variables|Default|GetQueue_List))
          (CallFunction|ResetQueueforGauntlet (.queue_number _returnvalue_5))
          (bind _output_get_4 (Variables|Default|SetWorld_State_ID (.world_state_id _returnvalue_5)))
          (bind _returnvalue_6 (Utilities|GetDataTableRow "/Game/Dialogue/Patient_Dialogue_Database.Patient_Dialogue_Database" _output_get_4)
            (:then
              (bind _output_get_5 (Variables|Default|SetDialogue_Options _returnvalue_6))
              (bind _returnvalue_7 (Actor|GetActorOfClass "/Game/Levels/in-level-things/Beastiary_Interaction.Beastiary_Interaction_C"))
              (Default|LoadAnimals _returnvalue_7 (.animal_list _output_get_5))))))))
  (Utilities|FlowControl|Sequence
    (:then_0
      ;[0.15 0.15 0.15 0.5] Load Different Parts of the World
      (bind _returnvalue_8 (WorldPartition|GetDataLayerManager))
      (switch name (Variables|Default|GetWorld_State_ID)
        (:Default
          (DataLayers|SetDataLayerRuntimeState _returnvalue_8 "/Game/Levels/Maps/DL_State_0.DL_State_0" "Unloaded" false :!class /Script/Engine.DataLayerManager :!label _label)
          (DataLayers|SetDataLayerRuntimeState _returnvalue_8 "/Game/Levels/Maps/DL_State_0_Perm.DL_State_0_Perm" "Activated" false :!class /Script/Engine.DataLayerManager)
          (DataLayers|SetDataLayerRuntimeState _returnvalue_8 "/Game/Levels/Maps/DL_State_1.DL_State_1" "Unloaded" false :!class /Script/Engine.DataLayerManager)
          (DataLayers|SetDataLayerRuntimeState _returnvalue_8 "/Game/Levels/Maps/DL_State_1-Perm.DL_State_1-Perm" "Activated" false :!class /Script/Engine.DataLayerManager)
          (DataLayers|SetDataLayerRuntimeState _returnvalue_8 "/Game/Levels/Maps/DL_State_2.DL_State_2" "Unloaded" false :!class /Script/Engine.DataLayerManager)
          (DataLayers|SetDataLayerRuntimeState _returnvalue_8 "/Game/Levels/Maps/DL_State_3.DL_State_3" "Activated" false :!class /Script/Engine.DataLayerManager))
        (:World_State_0
          (DataLayers|SetDataLayerRuntimeState _returnvalue_8 "/Game/Levels/Maps/DL_State_0.DL_State_0" "Activated" false :!class /Script/Engine.DataLayerManager)
          (DataLayers|SetDataLayerRuntimeState _returnvalue_8 "/Game/Levels/Maps/DL_State_0_Perm.DL_State_0_Perm" "Unloaded" false :!class /Script/Engine.DataLayerManager)
          (DataLayers|SetDataLayerRuntimeState _returnvalue_8 "/Game/Levels/Maps/DL_State_1.DL_State_1" "Unloaded" false :!class /Script/Engine.DataLayerManager)
          (DataLayers|SetDataLayerRuntimeState _returnvalue_8 "/Game/Levels/Maps/DL_State_1-Perm.DL_State_1-Perm" "Unloaded" false :!class /Script/Engine.DataLayerManager :!label _label_2)
          (DataLayers|SetDataLayerRuntimeState _returnvalue_8 "/Game/Levels/Maps/DL_State_2.DL_State_2" "Unloaded" false :!class /Script/Engine.DataLayerManager)
          (DataLayers|SetDataLayerRuntimeState _returnvalue_8 "/Game/Levels/Maps/DL_State_3.DL_State_3" "Unloaded" false :!class /Script/Engine.DataLayerManager))
        (:World_State_1
          (DataLayers|SetDataLayerRuntimeState _returnvalue_8 "/Game/Levels/Maps/DL_State_0.DL_State_0" "Unloaded" false :!class /Script/Engine.DataLayerManager)
          (DataLayers|SetDataLayerRuntimeState _returnvalue_8 "/Game/Levels/Maps/DL_State_0_Perm.DL_State_0_Perm" "Activated" false :!class /Script/Engine.DataLayerManager)
          (DataLayers|SetDataLayerRuntimeState _returnvalue_8 "/Game/Levels/Maps/DL_State_1.DL_State_1" "Activated" false :!class /Script/Engine.DataLayerManager)
          (goto _label_2))
        (:World_State_2
          (DataLayers|SetDataLayerRuntimeState _returnvalue_8 "/Game/Levels/Maps/DL_State_0.DL_State_0" "Unloaded" false :!class /Script/Engine.DataLayerManager)
          (DataLayers|SetDataLayerRuntimeState _returnvalue_8 "/Game/Levels/Maps/DL_State_0_Perm.DL_State_0_Perm" "Activated" false :!class /Script/Engine.DataLayerManager)
          (DataLayers|SetDataLayerRuntimeState _returnvalue_8 "/Game/Levels/Maps/DL_State_1.DL_State_1" "Unloaded" false :!class /Script/Engine.DataLayerManager)
          (DataLayers|SetDataLayerRuntimeState _returnvalue_8 "/Game/Levels/Maps/DL_State_1-Perm.DL_State_1-Perm" "Activated" false :!class /Script/Engine.DataLayerManager)
          (DataLayers|SetDataLayerRuntimeState _returnvalue_8 "/Game/Levels/Maps/DL_State_2.DL_State_2" "Activated" false :!class /Script/Engine.DataLayerManager)
          (DataLayers|SetDataLayerRuntimeState _returnvalue_8 "/Game/Levels/Maps/DL_State_3.DL_State_3" "Unloaded" false :!class /Script/Engine.DataLayerManager))
        (:World_State_3
          (goto _label))))
    (:then_1
      (bind _returnvalue_9 (UserInterface|CreateWidget "/Game/UI/Inventory/Timer_Widget.Timer_Widget_C"))
      (bind _output_get_6 (Variables|Default|Settimer_widget _returnvalue_9))
      (UserInterface|Viewport|AddtoViewport _output_get_6 0))))

(event EventTick
  (params (DeltaSeconds :type Float%20%28single-precision%29))
  (bind _returnvalue (Transformation|GetActorLocation))
  (bind _returnvalue_2 (Transformation|GetActorLocation))
  (bind _npc_queue (Variables|Default|GetNPC_Queue))
  (bind _death_count (Variables|Default|Getdeath_count))
  (bind _patient_sprite_names (Variables|Default|Getpatient_sprite_names))
  (bind _patient_sprite_names_2 (Variables|Default|Getpatient_sprite_names))
  (bind _npc_queue_2 (Variables|Default|GetNPC_Queue))
  (bind _npc_list (Variables|Default|GetNPC_List))
  (bind _npc_list_2 (Variables|Default|GetNPC_List))
  (bind _npc_queue_3 (Variables|Default|GetNPC_Queue))
  (bind _output (Utilities|Array|Get(acopy) _npc_queue))
  (bind _outitem (Utilities|Array|Random (.possible_animals _output)))
  (if (and (not (Utilities|IsValid (Variables|Default|Getend_of_level_ui))) (Variables|Default|Getday_finished))
    (Variables|Default|Setday_started false)
    (Variables|Default|Setday_finished false)
    (if (< _death_count (Variables|Default|Getdeath_limit))
      (Utilities|FlowControl|Delay 0.7))
    (bind _returnvalue_3 (UserInterface|CreateWidget "/Game/UI/End-Of-Level/BP_End_of_level_popup.BP_End_of_level_popup_C" 0 0 _death_count (Variables|Default|Getcure_count) (Math|Float|Truncate (Variables|Default|GetTime_Since_Start)) (Variables|Default|Getdeath_limit) (Variables|Default|Getday%20count)))
    (bind _output_get (Variables|Default|Setend_of_level_ui _returnvalue_3))
    (UserInterface|Viewport|AddtoViewport _output_get 0)
    (CallFunction|StopTimer)
    (elif (Variables|Default|Getday_started)
      (Utilities|FlowControl|Sequence
        (:then_0
          ;[0.15 0.15 0.15 0.5] Create backlog of NPC's to Spawn
          (for _array_element _npc_list
            (if (<= (.Spawn_Time (Utilities|Struct|BreakNPC_Spawn_Config_Struct _array_element)) (Variables|Default|GetPatient_Spawn_Time))
              (Utilities|Array|Add (Variables|Default|GetNPC_Queue) _array_element)
              (Utilities|Array|RemoveItem _npc_list _array_element))))
        (:then_1
          ;[0.15 0.15 0.15 0.5] Determine if a new NPC can be spawned
          (if (Variables|Default|GetCanSpawnNewPatient)
            (if (> (Utilities|Array|Length (Variables|Default|GetNPC_Queue)) 0)
              ;[0.15 0.15 0.15 0.5] Pick Random Animal and dialogue for Patient
              (if (and (.first_patient_of_day _output) (> (Variables|Default|Gettemp_gauntlet_time_increase) 0))
                (bind _output_get_2 (Variables|Default|Setday%20count (+ (Variables|Default|Getday%20count) 1)))
                (Variables|Default|Setdeath_limit (+ (Variables|Default|Getdeath_limit) 1))
                (Default|ShowNewDayTitle (Variables|Default|Gettimer_widget) _output_get_2))
              (if (.special_npc _output)
                (bind _output_get_3 (Variables|Default|SetTemp_animal_name _outitem))
                (bind _returnvalue_4 (Utilities|GetDataTableRow "/Game/Characters/Patients/Special_Patient_Database.Special_Patient_Database" (Utilities|String|StringToName (.special_npc_type _output)))
                  (:then
                    (Development|PrintString _output_get_3)
                    ;[0.15 0.15 0.15 0.5] Spawn New Special NPC
                    (bind _returnvalue_5 (Game|SpawnActorfromClass "/Game/Characters/Patients/BP_Special_Patient_Template.BP_Special_Patient_Template_C" (Math|Transform|MakeTransform _returnvalue "0, 0, 0" "1.000000,1.000000,1.000000") "Undefined" "MultiplyWithRoot" 0 _returnvalue "0.000000,0.000000,0.000000" false 0.0 0.0 0 0 "0.000000,0.000000,0.000000" (Utilities|String|ParseIntoArray (Utilities|String|ToString(Text) (.OutItem (Utilities|Array|Random (.difficulty_to_dialogue (.Value (Utilities|Map|Find (.animals _returnvalue_4) _output_get_3)))))) "///" false) _output_get_3 (Utilities|Text|ToText(String) (.name _returnvalue_4)) (.sprite _returnvalue_4) 0))
                    (Audio|PlaySound2D "/Game/Assets/Sounds/bell-98033.bell-98033" 1.0 1.0 0.0 0 0)
                    ;;[0.15 0.15 0.15 0.5] Determine NPC spawn location and which QUEUE to go to.
                    (bind _array_element_2 (Utilities|Array|ForEachLoopwithBreak (Variables|Default|GetQueue_List) :!label _label)
                      (:LoopBody
                        (if (not (Variables|/Game/Characters/Patients/BP_Queue.BP_Queue_C|Getin_Use _array_element_2))
                          (Default|MovetoLocation _returnvalue_5 (Transformation|GetWorldLocation (Variables|/Game/Characters/Patients/BP_Queue.BP_Queue_C|GetStart _array_element_2)))
                          (Variables|/Game/Characters/Patients/BP_Queue.BP_Queue_C|Setin_Use _array_element_2 true)
                          (Variables|/Game/Characters/Patients/BP_Patient_Template.BP_Patient_Template_C|Setqueue _returnvalue_5 _array_element_2)
                          (Variables|/Game/Characters/Patients/BP_Patient_Template.BP_Patient_Template_C|SetspawnLocation _returnvalue_5 (Transformation|GetActorLocation self))
                          (Utilities|Array|Add (Variables|Default|GetSpawned_Patients) _returnvalue_5)
                          (goto _label Break)))
                      (:Completed
                        ;;[0.7292 0.7292 0.7292 0.5] Update list of NPC's to Spawn
                        (Utilities|Array|RemoveItem _npc_queue_3 (Utilities|Array|Get(acopy) _npc_queue_3))
                        (Variables|Default|SetCanSpawnNewPatient (< (Utilities|Array|Length (Variables|Default|GetSpawned_Patients)) (Utilities|Array|Length (Variables|Default|GetQueue_List))))
                        (Development|PrintString "Spawned new Patient")))))
                (else
                  (bind _outrownames (DataTable|GetDataTableRowNames "/Game/Characters/Patients/Patient_Name_Database.Patient_Name_Database"))
                  (bind _output_get_4 (Variables|Default|SetTemp_animal_name _outitem))
                  (bind _returnvalue_6 (Utilities|GetDataTableRow "/Game/Characters/Patients/Patient_Name_Database.Patient_Name_Database" (.OutItem (Utilities|Array|Random _outrownames)))
                    (:then
                      ;;[0.15 0.15 0.15 0.5] Choose NPC Skin
                      (bind _outrownames_2 (DataTable|GetDataTableRowNames "/Game/Characters/Patients/Patient_Database.Patient_Database"))
                      (bind _output_get_5 (Variables|Default|Settemp_name (.OutItem (Utilities|Array|Random _outrownames_2))))
                      (while (Utilities|Array|ContainsItem _patient_sprite_names _output_get_5)
                        (bind _output_get_6 (Variables|Default|Settemp_name (.OutItem (Utilities|Array|Random _outrownames_2)))))
                      (Utilities|Array|Add _patient_sprite_names _output_get_6)
                      (if (> (Utilities|Array|Length _patient_sprite_names_2) 3)
                        (Utilities|Array|RemoveIndex _patient_sprite_names_2))
                      (bind _returnvalue_7 (Utilities|GetDataTableRow "/Game/Characters/Patients/Patient_Database.Patient_Database" _output_get_6)
                        (:then
                          ;[0.15 0.15 0.15 0.5] Spawn New NPC
                          (bind _returnvalue_8 (Game|SpawnActorfromClass "/Game/Characters/Patients/BP_Patient_Template.BP_Patient_Template_C" (Math|Transform|MakeTransform _returnvalue_2 "0, 0, 0" "1.000000,1.000000,1.000000") "Undefined" "MultiplyWithRoot" 0 _returnvalue_2 "0.000000,0.000000,0.000000" false 0.0 0.0 0 0 "0.000000,0.000000,0.000000" (Utilities|String|ParseIntoArray (Utilities|String|ToString(Text) (.OutItem (Utilities|Array|Random (.difficulty_to_dialogue (.Value (Utilities|Map|Find (.dialogue_per_animal (Variables|Default|GetDialogue_Options)) _output_get_4)))))) "///" false) _output_get_4 (.name _returnvalue_6) (.sprite _returnvalue_7) 0))
                          ;;[0.15 0.15 0.15 0.5] Determine NPC spawn location and which QUEUE to go to.
                          (Audio|PlaySound2D "/Game/Assets/Sounds/bell-98033.bell-98033" 1.0 1.0 0.0 0 0)
                          (bind _array_element_3 (Utilities|Array|ForEachLoopwithBreak (Variables|Default|GetQueue_List) :!label _label_2)
                            (:LoopBody
                              (if (not (Variables|/Game/Characters/Patients/BP_Queue.BP_Queue_C|Getin_Use _array_element_3))
                                (Default|MovetoLocation _returnvalue_8 (Transformation|GetWorldLocation (Variables|/Game/Characters/Patients/BP_Queue.BP_Queue_C|GetStart _array_element_3)))
                                (Variables|/Game/Characters/Patients/BP_Queue.BP_Queue_C|Setin_Use _array_element_3 true)
                                (Variables|/Game/Characters/Patients/BP_Patient_Template.BP_Patient_Template_C|Setqueue _returnvalue_8 _array_element_3)
                                (Variables|/Game/Characters/Patients/BP_Patient_Template.BP_Patient_Template_C|SetspawnLocation _returnvalue_8 (Transformation|GetActorLocation self))
                                (Utilities|Array|Add (Variables|Default|GetSpawned_Patients) _returnvalue_8)
                                (goto _label_2 Break)))
                            (:Completed
                              ;;[0.7292 0.7292 0.7292 0.5] Update list of NPC's to Spawn
                              (Utilities|Array|RemoveItem _npc_queue_2 (Utilities|Array|Get(acopy) _npc_queue_2))
                              (Variables|Default|SetCanSpawnNewPatient (< (Utilities|Array|Length (Variables|Default|GetSpawned_Patients)) (Utilities|Array|Length (Variables|Default|GetQueue_List))))
                              (Development|PrintString "Spawned new Patient")))))))))
              (elif (and (> (Utilities|Array|Length _npc_list_2) 0) (== (Utilities|Array|Length (Variables|Default|GetSpawned_Patients)) 0))
                (Variables|Default|SetPatient_Spawn_Time (+ (- (- (.spawn_time (Utilities|Array|Get(acopy) _npc_list_2)) (Variables|Default|GetPatient_Spawn_Time)) 1.0) (Variables|Default|GetPatient_Spawn_Time)))
                (else
                  ;[0.15 0.15 0.15 0.5] End Day when no more patients left
                  (if (and (== (Utilities|Array|Length _npc_list_2) 0) (== (Utilities|Array|Length (Variables|Default|GetSpawned_Patients)) 0))
                    (Variables|Default|Setday_finished true)))))))))))

(fn ConstructionScript)