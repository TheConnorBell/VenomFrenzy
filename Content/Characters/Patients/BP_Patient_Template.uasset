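; Flipbook patient template: a bitten NPC that queues, talks and awaits matching antivenom before a death timer expires.
; Tick runs an integer MovementState machine, lerping swaying walks between queue points and spawn, and updates the countdown widget.
; Giveitem stops the timer on a correct cure; venom kills immediately, other wrong items kill after leaving the queue.
; Death plays a tipping timeline and bell, spawns a corpse and notifies BP_Patient_Spawner.
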(event OnComponentEndOverlap(InteractBox)
  (params (OverlappedComponent :type Primitive%20Component%20Object%20Reference) (OtherActor :type Actor%20Object%20Reference) (OtherComp :type Primitive%20Component%20Object%20Reference) (OtherBodyIndex :type Integer))
  ;[0.15 0.15 0.15 0.5] Close Dialogue if player walks away
  (bind _asbp_player_character (Utilities|Casting|CastToBP_PlayerCharacter OtherActor))
  (Utilities|IsValid _asbp_player_character
    (:Is%20Valid
      (Utilities|IsValid (Variables|Default|GetUI)
        (:Is%20Valid
          (Widget|RemovefromParent (Variables|Default|GetUI))
          (Variables|Default|SetUI 0)
          (Variables|Default|Setdialogue_index -1))))))

(event Custom|MoveToLocation
  (params (Destination :type Vector))
  (bind _output_get (Variables|Default|SetdestinationLocation Destination))
  (Variables|Default|SetelapsedTime 0.0)
  (Variables|Default|SettravelTime (/ (Math|Vector|VectorLength (- _output_get (Variables|Default|GetstartLocation))) 3e+02))
  (Variables|Default|SetisMoving true)
  ;[1 0 0 0.5] Start Death Timer, Need to actually decide on whether this is constant, or variable
  (if (not (Variables|Default|GetdeathTimerStarted))
    (Utilities|Time|SetTimerbyFunctionName 0 "PatientDeathTimer" (Variables|Default|Getdefault_death_time))
    (Variables|Default|SetdeathTimerStarted true)))

(event Custom|PatientDeath
  (bind _alpha (Timeline|DeathTimeline Play)
    (:Update
      (Transformation|SetActorRotation (Math|Rotator|MakeRotator (* _alpha -9e+01) 0.0 0.0)))
    (:Finished
      (Variables|Default|SetmovementState 5) ; Die
      (Audio|PlaySound2D "/Game/Assets/Sounds/single-church-bell-2-352062.single-church-bell-2-352062" 1.0 1.0 0.0 0 0))))

(event Custom|Give%20item
  (params (item_id :type String))
  (if (Utilities|Enum|Equal(Enum) (Utilities|String|Append (Variables|Default|GetAnimal_That_Bit_Patient) "-antivenom") item_id)
    (Utilities|Time|ClearTimerbyFunctionName 0 "PatientDeathTimer")
    (Variables|Default|SetmovementState 3) ; Walk away after getting item
    (if (not (Variables|Default|Getsent_cure_message))
      (bind _outactors (Actor|GetAllActorsOfClass "/Game/Characters/Patients/BP_Patient_Spawner.BP_Patient_Spawner_C"))
      (Default|PatientDealtwith (Utilities|Array|Get(acopy) _outactors) true)
      (Variables|Default|Setsent_cure_message true))
    (elif (Utilities|Enum|Equal(Enum) (.RightS (Utilities|String|Split item_id "-")) "venom")
      (Variables|Default|SetmovementState 6) ; Die
      (else
        (Variables|Default|SetmovementState 3) ; Die
        (Variables|Default|Setis_about_to_die true)))))

(event Custom|startSwaying
  (bind _newtrack_0 (Timeline|ContinousSwayingTimeline Play)
    (:Update
      (Transformation|SetActorRotation (Math|Rotator|MakeRotator 0.0 (* _newtrack_0 1e+01) 0.0)))
    (:Finished
      (if (Variables|Default|GetisMoving)
        (Timeline|ContinousSwayingTimeline PlayFromStart)))))

(event Custom|PatientDeathTimer
  ;[1 0 0 0.5] Start Death Timer, Need to actually decide on whether this is constant, or variable
  (Variables|Default|SetmovementState 6) ; Die
)

(event EventBeginPlay
  (Sprite|SetFlipbook (Variables|Default|GetPaperFlipbook) (Variables|Default|GetPatient_Sprite)))

(event EventTalk
  ;[0.6706 0.1137 0.1137 0.502] Comment
  (Math|Integer|IncrementInt (Variables|Default|Getdialogue_index)
    (:%20%20
      (if (< (Variables|Default|Getdialogue_index) (Utilities|Array|Length (Variables|Default|Getdialogue)))
        ;[0.6706 0.1137 0.1137 0.502] Show next dialogue line
        (Variables|Default|GetUI
          (:then
            _)
          (:else
            (bind _returnvalue (UserInterface|CreateWidget "/Game/UI/Dialogue/BP_Dialogue_Widget.BP_Dialogue_Widget_C"))
            (bind _output_get (Variables|Default|SetUI _returnvalue))
            (UserInterface|Viewport|AddtoViewport _output_get 0)))
        (Rendering|Components|TextRender|SetText (Variables|/Game/UI/Dialogue/BP_Dialogue_Widget.BP_Dialogue_Widget_C|GetDialogueText (Variables|Default|GetUI)) (Utilities|Text|ToText(String) (Utilities|Array|Get(acopy) (Variables|Default|Getdialogue) (Variables|Default|Getdialogue_index))))
        (Rendering|Components|TextRender|SetText (Variables|/Game/UI/Dialogue/BP_Dialogue_Widget.BP_Dialogue_Widget_C|GetPatientName (Variables|Default|GetUI)) (Variables|Default|Getname))
        (else
          ;[0.6706 0.1137 0.1137 0.502] Remove Dialogue window, and make person walk away. (TODO: Update to allow giving antivenom
          (Widget|RemovefromParent (Variables|Default|GetUI))
          (Variables|Default|SetUI 0)
          (Variables|Default|Setdialogue_index -1))))))

(event EventTick
  (params (DeltaSeconds :type Float%20%28single-precision%29))
  (bind _returnvalue (Class|KismetSystemLibrary|GetTimerRemainingTime 0 "PatientDeathTimer"))
  (bind _returnvalue_2 (Transformation|GetActorLocation))
  (bind _widget (Variables|Default|GetWidget))
  (bind _ui (Variables|Default|GetUI))
  (bind _default_death_time (Variables|Default|Getdefault_death_time))
  (bind _returnvalue_3 (Math|Float|Round _returnvalue))
  (bind _returnvalue_4 (/ _returnvalue _default_death_time))
  (bind _returnvalue_5 (- 1.0 _returnvalue_4))
  (bind _returnvalue_6 (/ _returnvalue_3 60))
  (Utilities|FlowControl|Sequence
    (:then_0
      (if (Variables|Default|GetisMoving)
        (CallFunction|StartSwaying)
        (if (Utilities|Operators|EqualEqual (Transformation|GetActorLocation) (Variables|Default|GetdestinationLocation) 0.1)
          (Variables|Default|SetisMoving false)
          (Variables|Default|SetmovementState (+ (Variables|Default|GetmovementState) 1))
          (else
            (bind _output_get (Variables|Default|SetelapsedTime (+ DeltaSeconds (Variables|Default|GetelapsedTime))))
            (Transformation|SetActorLocation (Math|Vector|Lerp(Vector) (Variables|Default|GetstartLocation) (Variables|Default|GetdestinationLocation) (Math|Float|Clamp(Float) (/ _output_get (Variables|Default|GettravelTime)))) false false)))
        (else
          (switch int (Variables|Default|GetmovementState)
            (:1
              (Variables|Default|SetstartLocation (Variables|Default|GetdestinationLocation))
              (CallFunction|MovetoLocation (Transformation|GetWorldLocation (Variables|/Game/Characters/Patients/BP_Queue.BP_Queue_C|GetEnd (Variables|Default|Getqueue)))))
            (:3
              (Variables|Default|SetstartLocation (Variables|Default|GetdestinationLocation))
              (CallFunction|MovetoLocation (Transformation|GetWorldLocation (Variables|/Game/Characters/Patients/BP_Queue.BP_Queue_C|GetStart (Variables|Default|Getqueue)))))
            (:4
              (if (Variables|Default|Getis_about_to_die)
                (Variables|Default|SetmovementState 6) ; Die
                (else
                  (Variables|Default|SetstartLocation (Variables|Default|GetdestinationLocation))
                  (CallFunction|MovetoLocation (Variables|Default|GetspawnLocation)))))
            (:5
              (bind _returnvalue_7 (Actor|GetActorOfClass "/Game/Characters/Patients/BP_Patient_Spawner.BP_Patient_Spawner_C"))
              (Utilities|Array|RemoveItem (Variables|/Game/Characters/Patients/BP_Patient_Spawner.BP_Patient_Spawner_C|GetSpawned_Patients _returnvalue_7) self)
              (Variables|/Game/Characters/Patients/BP_Patient_Spawner.BP_Patient_Spawner_C|SetCanSpawnNewPatient _returnvalue_7 true)
              (Variables|/Game/Characters/Patients/BP_Queue.BP_Queue_C|Setin_Use (Variables|Default|Getqueue) false)
              (Game|SpawnActorfromClass "/Game/Characters/Patients/BP_Dead_Patient.BP_Dead_Patient_C" (Math|Transform|MakeTransform (Math|Vector|MakeVector (.x _returnvalue_2) (.y _returnvalue_2) (- (.z _returnvalue_2) 2e+02))) "Undefined" "MultiplyWithRoot" 0 0.0 0)
              (if (not (Variables|Default|Getsent_cure_message))
                (bind _outactors (Actor|GetAllActorsOfClass "/Game/Characters/Patients/BP_Patient_Spawner.BP_Patient_Spawner_C"))
                (Default|PatientDealtwith (Utilities|Array|Get(acopy) _outactors) false)
                (Variables|Default|Setsent_cure_message true)
                (Actor|DestroyActor self)))
            (:6
              (Utilities|IsValid _ui :!label _label
                (:Is%20Valid
                  (Widget|RemovefromParent _ui))
                (:Is%20Not%20Valid
                  _))
              (CallFunction|PatientDeath))
            (:7
              (goto _label))))))
    (:then_1
      (if (Variables|Default|GetdeathTimerStarted)
        (Utilities|IsValid _widget
          (:Is%20Valid
            (bind _aspatient_death_timer_widget (Utilities|Casting|CastToPatient_Death_Timer_Widget (UserInterface|GetWidget _widget)))
            (Utilities|IsValid _aspatient_death_timer_widget
              (:Is%20Valid
                (if (> _returnvalue_6 0)
                  (Default|UpdateTimer _aspatient_death_timer_widget (Utilities|Text|ToText(String) (Utilities|String|Append (Utilities|String|ToString(Integer) _returnvalue_6) ":" (Utilities|String|ToString(Text) (Utilities|Text|ToText(Integer) (Math|Integer|%(Integer) _returnvalue_3 60) false true 2)))) _returnvalue_5)
                  (else
                    (Default|UpdateTimer _aspatient_death_timer_widget (Utilities|Text|ToText(Integer) _returnvalue_3) _returnvalue_5)))))))))))

(fn ConstructionScript)